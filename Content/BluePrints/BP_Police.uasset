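; BP_Police is a police-themed Blueprint that spins a red light and a blue light.
; Each Tick reads each light's world yaw and adds RotateSpeed, with no delta-time scaling.
; The result is written through SetRelativeLocationAndRotation, which also receives the light's world location as its relative location.
; The construction script and RotateLight function are empty.
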(event `self.ReceiveTick`
  (params (DeltaSeconds :type "Float (single-precision)"))
  (bind (_returnvalue_roll _returnvalue_pitch _returnvalue_yaw) (`KismetMathLibrary.BreakRotator` (`SceneComponent.K2_GetComponentRotation` (`self.bluelight`))))
  (bind (_returnvalue_roll_2 _returnvalue_pitch_2 _returnvalue_yaw_2) (`KismetMathLibrary.BreakRotator` (`SceneComponent.K2_GetComponentRotation` (`self.redlight`))))
  (bind _result (`/Engine/EditorBlueprintResources/StandardMacros.IncrementFloat` _returnvalue_yaw_2)
    (:`  `
      (`SceneComponent.K2_SetRelativeLocationAndRotation` (`self.redlight`) (`SceneComponent.K2_GetComponentLocation` (`self.redlight`)) (`KismetMathLibrary.MakeRotator` 0.0 0.0 (+ (`self.rotateSpeed`) _result)) false false)
      (bind _result_2 (`/Engine/EditorBlueprintResources/StandardMacros.IncrementFloat` _returnvalue_yaw)
        (:`  `
          (`SceneComponent.K2_SetRelativeLocationAndRotation` (`self.bluelight`) (`SceneComponent.K2_GetComponentLocation` (`self.bluelight`)) (`KismetMathLibrary.MakeRotator` 0.0 0.0 (+ (`self.rotateSpeed`) _result_2)) false false))))))

(fn `RotateLight`)

(fn `UserConstructionScript`)