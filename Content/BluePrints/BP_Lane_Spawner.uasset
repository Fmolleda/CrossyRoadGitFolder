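; BP_Lane_Spawner spawns a chain of randomized BP_Lane actors, starting just below the player pawn.
; On BeginPlay, SpawnInitialLanes places the first lane, then attaches each following one at the newest lane's SpawnPoint.
; SpawnLane tracks the newest lane, gives it a reference back to the spawner and calls its RandomizeLane.
; SpawnLaneAtSpawnPoint extends the chain by one lane.
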(event `self.ReceiveBeginPlay`
  (`self.SpawnInitialLanes`))

(fn `SpawnInitialLanes`
  (bind (_returnvalue_x _returnvalue_y _returnvalue_z) (`KismetMathLibrary.BreakVector` (`self.K2_GetActorLocation` (`GameplayStatics.GetPlayerPawn` 0))))
  (for _ (range 4)
    (`/Engine/EditorBlueprintResources/StandardMacros.IsValid` (`self.NewestLane`)
      (:`Is Valid`
        (`self.SpawnLaneAtSpawnPoint`))
      (:`Is Not Valid`
        (`self.SpawnLane` (`KismetMathLibrary.MakeVector` _returnvalue_x _returnvalue_y (`KismetMathLibrary.Conv_IntToDouble` (+ _returnvalue_z -50))))))))

(fn `SpawnLane`
  (params (SpawnLocation :type "Vector Structure"))
  (bind _returnvalue (`|SpawnActorFromClass` "/Game/BluePrints/BP_Lane.BP_Lane_C" (`KismetMathLibrary.MakeTransform` SpawnLocation) "Undefined" "OverrideRootScale" null null))
  (bind _output_get (set `self.NewestLane` _returnvalue))
  (set `/Game/BluePrints/BP_Lane.LaneSpawner` self _output_get)
  (`/Game/BluePrints/BP_Lane.RandomizeLane` _output_get))

(fn `SpawnLaneAtSpawnPoint`
  (`self.SpawnLane` (`SceneComponent.K2_GetComponentLocation` (`/Game/BluePrints/BP_Lane.SpawnPoint` (`self.NewestLane`)))))

(fn `UserConstructionScript`)