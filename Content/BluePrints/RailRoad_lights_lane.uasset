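; Railroad signal light Blueprint that alternately flashes a left and a right light.
; Event Tick branches on LeftLightOn, raises that side's intensity, then a one-second Delay switches it off and flips the flag to hand over to the other side.
; The loop relies on the latent Delay inside Tick for pacing and runs continuously, with no external trigger.
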(event `self.ReceiveTick`
  (params (DeltaSeconds :type "Float (single-precision)"))
  (if (`self.Left light On`)
    (`LightComponent.SetIntensity` (`self.Left_light`) 10000.0)
    (`KismetSystemLibrary.Delay` 1.0)
    (`LightComponent.SetIntensity` (`self.Left_light`) 0.0)
    (set `self.Left light On` false)
    (else
      (`LightComponent.SetIntensity` (`self.Right_light`) 10000.0)
      (`KismetSystemLibrary.Delay` 1.0)
      (`LightComponent.SetIntensity` (`self.Right_light`) 0.0)
      (set `self.Left light On` true))))

(fn `UserConstructionScript`)