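; BP_Car is a car actor that drives forward on its own and brakes for chickens.
; Each tick it moves a fixed, frame-rate-dependent step along its forward vector without sweeping, unless StopCar is set.
; When a BP_Chicken begins overlapping the Safety_box component, it sets StopCar and plays a brake sound at the car's location.
; Nothing in this Blueprint clears StopCar, so the car stays stopped afterward.
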(event `self.ReceiveTick`
  (params (DeltaSeconds :type "Float (single-precision)"))
  (if (`self.StopCar`)
    (`self.K2_SetActorLocation` (`self.K2_GetActorLocation`))
    (else
      (`self.K2_SetActorLocation` (+ (`self.K2_GetActorLocation`) (* (`self.GetActorForwardVector`) 4))))))

(event `self.Safety_box.OnComponentBeginOverlap`
  (params (OverlappedComponent :type "PrimitiveComponent Object Reference") (OtherActor :type "Actor Object Reference") (OtherComp :type "PrimitiveComponent Object Reference") (OtherBodyIndex :type Integer) (bFromSweep :type Boolean) (SweepResult :type "HitResult Structure (by ref)"))
  (cast `/Game/BluePrints/BP_Chicken` OtherActor)
  (set `self.StopCar` true)
  (`GameplayStatics.PlaySoundAtLocation` "/Game/Sounds/SoundCues/Car_Brakes.Car_Brakes" (`self.K2_GetActorLocation`) (struct) 1.0 1.0 0.0 null null null null))

(fn `UserConstructionScript`)