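; Player chicken character with axis-driven world-space movement, jumping with a sound, and a score for lanes passed through.
; On BeginPlay it loads the lane high score from a save slot if present, then creates the UI_HUB widget and hands it a self reference.
; Each BP_Lane overlap increments the counter and updates the HUD.
; Matching or beating the high score immediately saves it through ScoreSaver, creating the save if missing.
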(event `self.ReceiveBeginPlay`
  (bind _slotnameinchicken (`self.SlotNameInChicken`))
  ;[1 1 1] Load In Highscore
  (bind _returnvalue (`GameplayStatics.DoesSaveGameExist` _slotnameinchicken))
  (if _returnvalue
    (bind _returnvalue_2 (`GameplayStatics.LoadGameFromSlot` _slotnameinchicken))
    (bind _asscore_saver (cast `/Game/ScoreSaver` _returnvalue_2))
    (set `self.LaneHighScoreInChicken` (`/Game/ScoreSaver.LaneHighScore` _asscore_saver)))
  ;[1 1 1] UI Widget
  (bind _returnvalue_3 (`|CreateWidget` "/Game/UI_HUB.UI_HUB_C"))
  (`UserWidget.AddToViewport` _returnvalue_3 0)
  (set `/Game/UI_HUB.BPChicken` self _returnvalue_3)
  (set `self.UI HUB In Chicken` _returnvalue_3))

(event `InputAxis|Move Right / Left`
  (params (AxisValue :type "Float (single-precision)"))
  ;[1 1 1] Movement
  (`self.AddMovementInput` (0.0 90.0 0.0) AxisValue))

(event `InputAxis|Move Forward / Back`
  (params (AxisValue :type "Float (single-precision)"))
  ;[1 1 1] Movement
  (`self.AddMovementInput` (90.0 0.0 0.0) AxisValue))

(event `InputAction|Jump Action`
  (params (Key :type "Key Structure"))
  ;[1 1 1] Movement
  (:`Pressed`
    (`self.Jump`)
    (`GameplayStatics.PlaySoundAtLocation` "/Game/Sounds/SoundCues/Jump_sound.Jump_sound" (`self.K2_GetActorLocation`) (struct) 1.0 1.0 0.0 null null null null))
  (:`Released`
    (`self.StopJumping`)))

(event `self.ReceiveActorBeginOverlap`
  (params (OtherActor :type "Actor Object Reference"))
  ;[1 1 1] Count Lanes passed through for score
  (cast `/Game/BluePrints/BP_Lane` OtherActor)
  (bind _result (`/Engine/EditorBlueprintResources/StandardMacros.IncrementInt` (`self.LaneCounter`))
    (:`  `
      (bind _output_get (set `self.LaneCounter` _result))
      (`/Game/UI_HUB.Increase Lane counter` (`self.UI HUB In Chicken`))
      ;[1 1 1] If current score greater than highscore increase highscore
      (if (>= _output_get (`self.LaneHighScoreInChicken`))
        (bind _output_get_2 (set `self.LaneHighScoreInChicken` _output_get))
        ;[1 1 1] if save game exsist load it if not create one
        (bind _returnvalue (`GameplayStatics.DoesSaveGameExist` (`self.SlotNameInChicken`)))
        (if _returnvalue
          (bind _returnvalue_2 (`GameplayStatics.LoadGameFromSlot` (`self.SlotNameInChicken`)))
          ;[1 1 1] update highscroe save game
          (bind _output_get_3 (set `self.SaveGameSubclassInChicken` _returnvalue_2))
          (bind _asscore_saver (cast `/Game/ScoreSaver` _output_get_3))
          (set `/Game/ScoreSaver.LaneHighScore` _output_get_2 _asscore_saver)
          (`GameplayStatics.SaveGameToSlot` (`self.SaveGameSubclassInChicken`) (`self.SlotNameInChicken`))
          (else
            (bind _returnvalue_3 (`GameplayStatics.CreateSaveGameObject` "/Game/ScoreSaver.ScoreSaver_C"))
            (bind _output_get_4 (set `self.SaveGameSubclassInChicken` _returnvalue_3))
            (bind _asscore_saver_2 (cast `/Game/ScoreSaver` _output_get_4))
            (set `/Game/ScoreSaver.LaneHighScore` _output_get_2 _asscore_saver_2)
            (`GameplayStatics.SaveGameToSlot` (`self.SaveGameSubclassInChicken`) (`self.SlotNameInChicken`))))))))

(fn `UserConstructionScript`)